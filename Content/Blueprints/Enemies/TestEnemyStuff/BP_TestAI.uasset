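; Test enemy AI that wanders between random reachable points and moves toward pawns it sees, or toward the player when damaged and still alive.
; An attack collision overlap starts a delayed, repeating damage loop on the player while touching; the overlap checks only cast the player character, not the overlapping actor.
; Incoming damage lowers clamped health, calls a health update and destroys the enemy at zero, with debug prints throughout.
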(event OnSeePawn(PawnSensing)
  (params (Pawn :type Pawn%20Object%20Reference))
  (AI|AIMoveTo self "0, 0, 0" Pawn 5.0 false))

(event OnComponentBeginOverlap(AttackCollision)
  (params (OverlappedComponent :type Primitive%20Component%20Object%20Reference) (OtherActor :type Actor%20Object%20Reference) (OtherComp :type Primitive%20Component%20Object%20Reference) (OtherBodyIndex :type Integer) (bFromSweep :type Boolean) (SweepResult :type Hit%20Result%20Structure%20%28by%20ref%29))
  ;[0.15 0.15 0.15 0.5] Checks to see if touching player for attack
  (Utilities|Casting|CastToBP_FirstPersonCharacter (Game|GetPlayerCharacter 0))
  (Variables|Default|SetIsTouching? true)
  (CallFunction|AIAttack))

(event OnComponentEndOverlap(AttackCollision)
  (params (OverlappedComponent :type Primitive%20Component%20Object%20Reference) (OtherActor :type Actor%20Object%20Reference) (OtherComp :type Primitive%20Component%20Object%20Reference) (OtherBodyIndex :type Integer))
  ;[0.15 0.15 0.15 0.5] Checks to see if touching player for attack
  (Utilities|Casting|CastToBP_FirstPersonCharacter (Game|GetPlayerCharacter 0))
  (Variables|Default|SetIsTouching? false))

(event Custom|AIMove
  (AI|AIMoveTo self (.RandomLocation (AI|Navigation|GetRandomReachablePointinRadius (Transformation|GetActorLocation) 2e+03 0 0)) 0 5.0 false
    (:OnSuccess
      (CallFunction|AIMove))))

(event Custom|AI%20Attack
  ;[0.15 0.15 0.15 0.5] Enemy Attack - It works but needs improvment
  (if (Variables|Default|GetIsTouching?)
    (Utilities|FlowControl|Delay 1.0)
    (Game|Damage|ApplyDamage (Game|GetPlayerCharacter 0) 2e+01 0 0)
    (Utilities|FlowControl|Delay 3.0)
    (Development|PrintString "YesAttack")
    (CallFunction|AIAttack)
    (else
      (Utilities|FlowControl|Delay 0.5)
      (Development|PrintString "NoAttack"))))

(event Custom|Testing
  (Development|PrintString "Hiding"))

(event EventBeginPlay
  (CallFunction|AIMove))

(event Collision|EventActorBeginOverlap
  (params (OtherActor :type Actor%20Object%20Reference)))

(event EventTick
  (params (DeltaSeconds :type Float%20%28single-precision%29)))

(event Game|Damage|EventAnyDamage
  (params (Damage :type Float%20%28single-precision%29) (DamageType :type Damage%20Type%20Object%20Reference) (InstigatedBy :type Controller%20Object%20Reference) (DamageCauser :type Actor%20Object%20Reference))
  ;[0.15 0.15 0.15 0.5] Enemy Health
  (bind _output_get (Variables|Default|SetCurrentHealth (Math|Float|Clamp(Float) (- (Variables|Default|GetCurrentHealth) Damage) 0.0 1e+02)))
  (Development|PrintString (Utilities|String|ToString(Float) _output_get))
  (Default|CallEHealthUpdate _output_get (Variables|Default|GetMaxHealth))
  (if (== _output_get 0.0)
    (Actor|DestroyActor)
    (Development|PrintString "Dead")
    (else
      (Development|PrintString "NotDead")
      (bind _asbp_first_person_character (Utilities|Casting|CastToBP_FirstPersonCharacter (Game|GetPlayerCharacter 0)))
      (AI|AIMoveTo self "0, 0, 0" _asbp_first_person_character 5.0 false))))

(fn ConstructionScript)