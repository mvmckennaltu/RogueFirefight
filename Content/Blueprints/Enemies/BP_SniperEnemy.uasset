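; BP_SniperEnemy is a stationary enemy that turns to face the player and fires projectiles on a long timer.
; Two self-calling delay loops from BeginPlay drive it: one snaps rotation toward the player, the other spawns BP_SniperEnemyProjectile at ProjectileSpawnLocation without sight checks.
; AnyDamage lowers clamped health, calls EHealthUpdate and destroys the actor at zero.
; Movement, pawn sensing and overlap melee logic are left unconnected.
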(event OnSeePawn(PawnSensing)
  (params (Pawn :type Pawn%20Object%20Reference)))

(event OnComponentBeginOverlap(Box)
  (params (OverlappedComponent :type Primitive%20Component%20Object%20Reference) (OtherActor :type Actor%20Object%20Reference) (OtherComp :type Primitive%20Component%20Object%20Reference) (OtherBodyIndex :type Integer) (bFromSweep :type Boolean) (SweepResult :type Hit%20Result%20Structure%20%28by%20ref%29))
  ;[0.15 0.15 0.15 0.5] Checks to see if touching player for attack
)

(event OnComponentEndOverlap(Box)
  (params (OverlappedComponent :type Primitive%20Component%20Object%20Reference) (OtherActor :type Actor%20Object%20Reference) (OtherComp :type Primitive%20Component%20Object%20Reference) (OtherBodyIndex :type Integer))
  ;[0.15 0.15 0.15 0.5] Checks to see if touching player for attack
)

(event Custom|AIMove)

(event Custom|AI%20Attack
  ;[0.15 0.15 0.15 0.5] Enemy Attack - It works but needs improvment
  (Utilities|FlowControl|Delay 2e+01)
  (Game|SpawnActorfromClass "/Game/Blueprints/BP_SniperEnemyProjectile.BP_SniperEnemyProjectile_C" (Transformation|GetWorldTransform (Variables|Default|GetProjectileSpawnLocation)) "AlwaysSpawn" "MultiplyWithRoot" 0 0)
  (Development|PrintString "Yes Attack")
  (CallFunction|AIAttack))

(event Custom|AiLook
  (Transformation|SetActorRotation (Math|Rotator|FindLookatRotation (Transformation|GetActorLocation) (Transformation|GetActorLocation (Game|Player|GetPlayerPawn 0))))
  (Utilities|FlowControl|Delay 0.1)
  (CallFunction|AiLook))

(event EventBeginPlay
  (CallFunction|AiLook)
  (CallFunction|AIAttack))

(event Collision|EventActorBeginOverlap
  (params (OtherActor :type Actor%20Object%20Reference)))

(event EventTick
  (params (DeltaSeconds :type Float%20%28single-precision%29)))

(event Game|Damage|EventAnyDamage
  (params (Damage :type Float%20%28single-precision%29) (DamageType :type Damage%20Type%20Object%20Reference) (InstigatedBy :type Controller%20Object%20Reference) (DamageCauser :type Actor%20Object%20Reference))
  ;[0.15 0.15 0.15 0.5] Enemy Health
  (bind _output_get (Variables|Default|SetCurrentHealth (Math|Float|Clamp(Float) (- (Variables|Default|GetCurrentHealth) Damage) 0.0 1e+02)))
  (Development|PrintString (Utilities|String|ToString(Float) _output_get))
  (Default|CallEHealthUpdate _output_get (Variables|Default|GetMaxHealth))
  (if (== _output_get 0.0)
    (Actor|DestroyActor)
    (Development|PrintString "Dead")
    (else
      (Development|PrintString "NotDead"))))

(fn ConstructionScript)