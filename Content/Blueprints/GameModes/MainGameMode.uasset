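; Game mode that builds a randomized mission in each level and runs progression through a series of maps.
; BeginPlay sorts spawner components by type, spawns shuffled enemies and items using GameInstance difficulty over spawner count, then picks Raid, Sabotage or Rescue (print-only).
; Completing Raid or Sabotage activates the level exit.
; LevelTransition raises difficulty and opens a different random map, or the victory screen once enough levels are completed.
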(event Custom|CalcEncounterValue
  ;[0.15 0.15 0.15 0.5] Calculates the encounter value
  (bind _outactors (Actor|GetAllActorsOfClass "/Game/Blueprints/Spawners/SingleSpawner.SingleSpawner_C"))
  (for _array_element _outactors
    (Utilities|Array|AppendArray (Variables|Default|GetAll%20Spawners) (Actor|GetComponentsByClass _array_element "/Game/Blueprints/Spawners/SpawnerComponent.SpawnerComponent_C")))
  (bind _output_get (Variables|Default|SetEncounterValue (Utilities|Array|Length (Variables|Default|GetAll%20Spawners))))
  (Development|PrintString (Utilities|String|Append (Utilities|String|MakeLiteralString "Encounter value: ") (Utilities|String|ToString(Integer) _output_get))))

(event Custom|SpawnRaidObjective
  (bind _raidobjectivespawners (Variables|Default|GetRaidObjectiveSpawners))
  ;[0.15 0.15 0.15 0.5] Spawns enemies and items based on the amount decided
  (Utilities|Array|Shuffle _raidobjectivespawners)
  (Default|SpawnRaidObjective (Utilities|Array|Get(acopy) _raidobjectivespawners)))

(event Custom|Spawn%20Sabotage%20Objectives
  (bind _sabotageobjectivespawners (Variables|Default|GetSabotageObjectiveSpawners))
  (bind _output_get (Variables|Default|SetSabotageObjectivesToSpawn (/ (Variables|Default|GetEncounterValue) 6)))
  (Utilities|Array|Shuffle _sabotageobjectivespawners)
  (for _index (range 0 (Math|Integer|Min(Integer) _output_get (Utilities|Array|Length _sabotageobjectivespawners)))
    (if (Utilities|IsValid (Utilities|Array|Get(acopy) _sabotageobjectivespawners _index))
      (Default|SpawnSabotageObjective (Utilities|Array|Get(acopy) _sabotageobjectivespawners _index)))))

(event Custom|Log%20Collected%20Sabotage%20Objective
  (bind _sabotageobjectivestospawn (Variables|Default|GetSabotageObjectivesToSpawn))
  (bind _result (Math|Integer|IncrementInt (Variables|Default|GetCollectCounter))
    (:%20%20
      (if (>= _result _sabotageobjectivestospawn)
        (CallFunction|ActivateLevelExit)
        (else
          (Development|PrintString (Utilities|String|Append (Utilities|String|Append (Utilities|String|Append (Utilities|String|MakeLiteralString "Listeners Placed: ") (Utilities|String|ToString(Integer) _result)) "/") (Utilities|String|ToString(Integer) _sabotageobjectivestospawn))))))))

(event Custom|Activate%20Level%20Exit
  (bind _returnvalue (Actor|GetActorOfClass "/Game/Blueprints/Progression/LevelExit.LevelExit_C"))
  (Rendering|SetVisibility (Variables|/Game/Blueprints/Progression/LevelExit.LevelExit_C|GetStaticMesh _returnvalue) true false)
  (Collision|SetCollisionEnabled (Variables|/Game/Blueprints/Progression/LevelExit.LevelExit_C|GetStaticMesh _returnvalue) "QueryOnly")
  (bind _foundwidgets (Widget|GetAllWidgetsOfClass "/Game/UI/UI_InGameUIStuff/Objective.Objective_C" true)))

(event Custom|LevelInclusionHack
  (Game|OpenLevel(byObjectReference) "/Game/FirstPerson/Lvl_FirstPerson.Lvl_FirstPerson")
  (Game|OpenLevel(byObjectReference) "/Game/DesertRaid.DesertRaid"))

(event Custom|Calc%20Difficulty
  (bind _itemdifficulty (Variables|Default|GetItemDifficulty))
  (bind _enemydifficulty (Variables|Default|GetEnemyDifficulty))
  ;[0.15 0.15 0.15 0.5] Determines the amount of enemies and items to spawn
  (Variables|Default|SetItemstoSpawn (/ (Math|Random|RandomIntegerinRange _itemdifficulty (- _itemdifficulty 10)) (Variables|Default|GetEncounterValue)))
  (bind _output_get (Variables|Default|SetEnemiestoSpawn (/ (Math|Random|RandomIntegerinRange _enemydifficulty (- _enemydifficulty 9)) (Variables|Default|GetEncounterValue))))
  (Development|PrintString (Utilities|String|Append (Utilities|String|MakeLiteralString "Spawned enemies: ") (Utilities|String|ToString(Integer) _output_get))))

(event Custom|Sort%20Spawners
  ;[0.15 0.15 0.15 0.5] Sorts the spawners by type
  (for _array_element (Variables|Default|GetAll%20Spawners)
    (switch Utilities|FlowControl|Switch|SwitchonSpawnerTypes (Variables|/Game/Blueprints/Spawners/SpawnerComponent.SpawnerComponent_C|GetSpawnerType _array_element)
      (:NewEnumerator0
        (Utilities|Array|Add (Variables|Default|GetItemSpawners) _array_element))
      (:NewEnumerator1
        (Utilities|Array|Add (Variables|Default|GetEnemySpawners) _array_element))
      (:NewEnumerator2
        (Utilities|Array|Add (Variables|Default|GetRaidObjectiveSpawners) _array_element))
      (:NewEnumerator3
        (Utilities|Array|Add (Variables|Default|GetSabotageObjectiveSpawners) _array_element))
      (:NewEnumerator4
        (Utilities|Array|Add (Variables|Default|GetRescueObjective%20Spawners) _array_element)))))

(event Custom|SpawnEnemiesatChosenPoints
  (bind _enemyspawners (Variables|Default|GetEnemySpawners))
  ;[0.15 0.15 0.15 0.5] Spawns enemies and items based on the amount decided
  (Variables|Default|SetSpawnCounter 0)
  (Utilities|Array|Shuffle (Variables|Default|GetEnemySpawners))
  (for _index (range 0 (Math|Integer|Min(Integer) (Variables|Default|GetEnemiestoSpawn) (Utilities|Array|Length _enemyspawners)))
    (if (Utilities|IsValid (Utilities|Array|Get(acopy) _enemyspawners _index))
      (Default|SpawnEnemy (Utilities|Array|Get(acopy) _enemyspawners _index)))))

(event Custom|SpawnItemsatChosenPoints
  (bind _itemspawners (Variables|Default|GetItemSpawners))
  ;[0.15 0.15 0.15 0.5] Spawns enemies and items based on the amount decided
  (Variables|Default|SetSpawnCounter 0)
  (Utilities|Array|Shuffle _itemspawners)
  (for _index (range 0 (Math|Integer|Min(Integer) (Variables|Default|GetItemstoSpawn) (Utilities|Array|Length _itemspawners)))
    (if (Utilities|IsValid (Utilities|Array|Get(acopy) _itemspawners _index))
      (Default|SpawnItem (Utilities|Array|Get(acopy) _itemspawners _index)))))

(event Custom|RaidObjectiveCollected
  (Variables|Default|SetObjectiveisFound true)
  (Development|PrintString "Objective Found!")
  (CallFunction|ActivateLevelExit))

(event Custom|Level%20Transition
  (bind _gamemaps (Variables|Default|GetGameMaps))
  (bind _output (Utilities|Array|Get(acopy) _gamemaps))
  (bind _returnvalue (Game|GetCurrentLevelName true))
  (Utilities|Array|Shuffle _gamemaps)
  (while (Utilities|Enum|Equal(Enum) _output _returnvalue)
    (Utilities|Array|Shuffle (Variables|Default|GetGameMaps)))
  (bind _ascross_level_data (Utilities|Casting|CastToCrossLevelData (Game|GetGameInstance)))
  (bind _result (Math|Integer|IncrementInt (Variables|/Game/Blueprints/GameModes/CrossLevelData.CrossLevelData_C|GetCurrentLevel _ascross_level_data))
    (:%20%20
      (if (> _result 3)
        (Game|OpenLevel(byObjectReference) "/Game/Levels/VictoryScreen.VictoryScreen")
        (else
          (Utilities|Array|Add (Variables|/Game/Blueprints/GameModes/CrossLevelData.CrossLevelData_C|GetCompleted%20Levels _ascross_level_data) _returnvalue)
          (Default|IncrementDifficulty _ascross_level_data)
          (Game|OpenLevel(byName) (Utilities|String|StringToName _output)))))))

(event Custom|SetDifficultyValues
  (bind _ascross_level_data (Utilities|Casting|CastToCrossLevelData (Game|GetGameInstance)))
  (Variables|Default|SetItemDifficulty (Variables|/Game/Blueprints/GameModes/CrossLevelData.CrossLevelData_C|GetItemDifficulty _ascross_level_data))
  (Variables|Default|SetEnemyDifficulty (Variables|/Game/Blueprints/GameModes/CrossLevelData.CrossLevelData_C|GetEnemyDifficulty _ascross_level_data)))

(event Custom|Choose%20Objective
  (bind _objectivetypes (Variables|Default|GetObjectiveTypes))
  (bind _enumvalue (|ForEachObjectiveTypes)
    (:LoopBody
      (Utilities|Array|Add _objectivetypes _enumvalue))
    (:then
      (Variables|Default|SetChosenObjective (.OutItem (Utilities|Array|Random _objectivetypes))))))

(event EventBeginPlay
  (Variables|Default|SetObjectiveisFound false)
  (CallFunction|CalcEncounterValue)
  ;[0.15 0.15 0.15 0.5] Ensures we don't break reality
  (if (> (Variables|Default|GetEncounterValue) 0)
    (CallFunction|SetDifficultyValues)
    (CallFunction|CalcDifficulty)
    (CallFunction|SortSpawners)
    (CallFunction|SpawnEnemiesatChosenPoints)
    (CallFunction|SpawnItemsatChosenPoints)
    (CallFunction|ChooseObjective)
    (switch Utilities|FlowControl|Switch|SwitchonObjectiveTypes (Variables|Default|GetChosenObjective)
      (:NewEnumerator0
        (CallFunction|SpawnRaidObjective)
        (Development|PrintString "Mission Type: Raid"))
      (:NewEnumerator1
        (Development|PrintString "Mission Type: Sabotage")
        (CallFunction|SpawnSabotageObjectives))
      (:NewEnumerator2
        (Development|PrintString "Mission Type: Rescue")))
    (else
      (Development|PrintString "Invalid Encounter Value!"))))

(event EventTick
  (params (DeltaSeconds :type Float%20%28single-precision%29)))

(fn ConstructionScript
  (|CallParentFunction))