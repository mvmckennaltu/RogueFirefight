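; Sniper enemy Blueprint that tracks its own health and dies when it runs out.
; Any damage lowers the clamped current health, then fires the EHealthUpdate dispatcher with current and max health.
; The actor destroys itself at zero health, with debug prints reporting health and death state.
; A SetWalkSpeed function sets the character movement's max walk speed.
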(event Game|Damage|EventAnyDamage
  (params (Damage :type Float%20%28single-precision%29) (DamageType :type Damage%20Type%20Object%20Reference) (InstigatedBy :type Controller%20Object%20Reference) (DamageCauser :type Actor%20Object%20Reference))
  ;[0.15 0.15 0.15 0.5] Enemy Health
  (bind _output_get (Variables|Default|SetCurrentHealth (Math|Float|Clamp(Float) (- (Variables|Default|GetCurrentHealth) Damage) 0.0 1e+02)))
  (Development|PrintString (Utilities|String|ToString(Float) _output_get))
  (Default|CallEHealthUpdate _output_get (Variables|Default|GetMaxHealth))
  (if (== _output_get 0.0)
    (Actor|DestroyActor)
    (Development|PrintString "Enemy Dead")
    (else
      (Development|PrintString "Enemy Not Dead"))))

(fn ConstructionScript)

(fn SetWalkSpeed
  (params (Speed :type Float%20%28double-precision%29))
  (Variables|/Script/Engine.CharacterMovementComponent|SetMaxWalkSpeed (Variables|Character|GetCharacterMovement) Speed))