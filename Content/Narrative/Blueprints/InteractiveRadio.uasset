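; InteractiveRadio is a narrative radio actor that plays an idle sound when play begins.
; An AudioEmitter component plays the IdleSound variable on BeginPlay.
; InteractSphere overlap events toggle the IsInteractable flag as an actor tagged Player enters or leaves, printing a debug message each time.
; The graph only tracks that flag and contains no interaction response.
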(event OnComponentBeginOverlap(InteractSphere)
  (params (OverlappedComponent :type Primitive%20Component%20Object%20Reference) (OtherActor :type Actor%20Object%20Reference) (OtherComp :type Primitive%20Component%20Object%20Reference) (OtherBodyIndex :type Integer) (bFromSweep :type Boolean) (SweepResult :type Hit%20Result%20Structure%20%28by%20ref%29))
  ;[0.15 0.15 0.15 0.5] Makes radio interactable when the player is near
  (if (Actor|ActorHasTag OtherActor "Player")
    (Variables|Default|SetIsInteractable true)
    (Development|PrintString "radio is interactable!")))

(event OnComponentEndOverlap(InteractSphere)
  (params (OverlappedComponent :type Primitive%20Component%20Object%20Reference) (OtherActor :type Actor%20Object%20Reference) (OtherComp :type Primitive%20Component%20Object%20Reference) (OtherBodyIndex :type Integer))
  ;[0.15 0.15 0.15 0.5] Turn of interact ability when player leaves the interact sphere
  (if (Actor|ActorHasTag OtherActor "Player")
    (Variables|Default|SetIsInteractable false)
    (Development|PrintString "radio is no longer interactable")))

(event EventBeginPlay
  ;[0.15 0.15 0.15 0.5] Sets the idle sound and starts playing it
  (Audio|Components|Audio|SetSound (Variables|Default|GetAudioEmitter) (Variables|Default|GetIdleSound))
  (Audio|Components|Audio|Play (Variables|Default|GetAudioEmitter) 0.0))

(event EventTick
  (params (DeltaSeconds :type Float%20%28single-precision%29)))

(fn ConstructionScript)